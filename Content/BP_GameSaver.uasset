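; BP_GameSaver manages the game's save data, including which fairies the player has befriended.
; It holds a BP_SaveFile object, loading it from its slot or saving a fresh one if none exists, and can delete the slot.
; Friend status lives in a fairy-keyed boolean map, and each change saves immediately if IsSavable is set.
; An all-friended check loops over the fairy enum, skipping None.
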(fn LoadSavefromMemory
  (bind _returnvalue (SaveGame|CreateSaveGameObject "/Game/BP_SaveFile.BP_SaveFile_C"))
  (bind _output_get (Variables|Default|SetSave%20State _returnvalue))
  (bind _returnvalue_2 (SaveGame|DoesSaveGameExist (Variables|/Game/BP_SaveFile.BP_SaveFile_C|GetSlotName _output_get) (Variables|/Game/BP_SaveFile.BP_SaveFile_C|GetUserIndex _output_get)))
  (if _returnvalue_2
    (bind _returnvalue_3 (SaveGame|LoadGamefromSlot (Variables|/Game/BP_SaveFile.BP_SaveFile_C|GetSlotName (Variables|Default|GetSave%20State)) (Variables|/Game/BP_SaveFile.BP_SaveFile_C|GetUserIndex (Variables|Default|GetSave%20State))))
    (bind _asbp_save_file (Utilities|Casting|CastToBP_SaveFile _returnvalue_3))
    (Variables|Default|SetSave%20State _asbp_save_file)
    (return)
    (else
      (CallFunction|SaveDatatoMemory)
      (return))))

(fn SaveDatatoMemory
  (bind _save_state (Variables|Default|GetSave%20State))
  (if (Variables|Default|GetIsSavable)
    (SaveGame|SaveGametoSlot _save_state (Variables|/Game/BP_SaveFile.BP_SaveFile_C|GetSlotName _save_state) (Variables|/Game/BP_SaveFile.BP_SaveFile_C|GetUserIndex _save_state))
    (return)))

(fn DeleteSaveData
  (bind _save_state (Variables|Default|GetSave%20State))
  (SaveGame|DeleteGameinSlot (Variables|/Game/BP_SaveFile.BP_SaveFile_C|GetSlotName _save_state) (Variables|/Game/BP_SaveFile.BP_SaveFile_C|GetUserIndex _save_state)))

(fn GetIsFriendswith
  (params (Fairy :type eFairy%20Enum :default "NewEnumerator3"))
  ;[1 1 1] Returns associated boolean with fairy name in Friends List
  (return (.Value (Utilities|Map|Find (Variables|/Game/BP_SaveFile.BP_SaveFile_C|GetFriendList (Variables|Default|GetSave%20State)) Fairy))))

(fn SetFairyasFriend
  (params (Fairy :type eFairy%20Enum :default "NewEnumerator3") (IsFriend :type Boolean))
  ;[1 1 1] Sets boolean friends list for the given fairy, and then saves to memory.
  (Utilities|Map|Add (Variables|/Game/BP_SaveFile.BP_SaveFile_C|GetFriendList (Variables|Default|GetSave%20State)) Fairy IsFriend)
  (CallFunction|SaveDatatoMemory))

(fn AllFairiesFriended
  (bind _enumvalue (|ForEacheFairy)
    (:LoopBody
      ;[1 1 1] Skip 'None' enum
      (if (Utilities|Enum|NotEqual(Enum) _enumvalue "NewEnumerator3")
        (bind _isfriend (CallFunction|GetIsFriendswith _enumvalue))
        (if (not _isfriend)
          (return false))))
    (:then
      (return true))))