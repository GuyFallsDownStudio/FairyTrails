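; BP_GPSLogger wraps the device's location services to hold the current latitude and longitude.
; GPSFirstTimeStartup initializes the services at navigation accuracy and starts them if that succeeds, setting the GPSIsOn flag accordingly.
; EnableGPS and DisableGPS start and stop the services and update that flag.
; RefreshLocation copies the last known location into Latitude and Longitude only when services are enabled and GPSIsOn is true.
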(fn RefreshLocation
  (bind _returnvalue (Class|LocationServices|AreLocationServicesEnabled))
  (if (and _returnvalue (Variables|Default|GetbGPSIsOn))
    ;[1 1 1] Refreshes Lat and Long only if location services are enabled and GPS is turned on internally.
    (bind _returnvalue_2 (Class|LocationServices|GetLastKnownLocation))
    (Variables|Default|SetLatitude (.Latitude (Utilities|Struct|BreakLocationServicesData _returnvalue_2)))
    (Variables|Default|SetLongitude (.Longitude (Utilities|Struct|BreakLocationServicesData _returnvalue_2)))
    (return)
    (else
      (return))))

(fn GPSFirstTimeStartup
  (bind _returnvalue (Class|LocationServices|InitLocationServices "LA_Navigation" 1e+03 0.0))
  (if _returnvalue
    (Class|LocationServices|StartLocationServices)
    (Variables|Default|SetbGPSIsOn true)
    (else
      (Variables|Default|SetbGPSIsOn false))))

(fn DisableGPS
  (Class|LocationServices|StopLocationServices)
  (Variables|Default|SetbGPSIsOn false))

(fn EnableGPS
  (Class|LocationServices|StartLocationServices)
  (Variables|Default|SetbGPSIsOn true))