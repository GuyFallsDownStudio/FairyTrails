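; BP_GPSChecker tests whether a player's GPS latitude and longitude fall inside a location's coordinate ranges.
; IsPlayerAtLocation passes the player coordinates and both location ranges to CalculateLocation and returns its result.
; CalculateLocation holds an in-range check on each axis, joined by AND, forming a simple bounding-box geofence.
; BreakCoordinateRanges extracts the minimum and maximum from a range's lower and upper bounds.
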(fn IsPlayeratLocation
  (params (LocationLatitudeRange :type Float%20Range%20Structure) (LocationLongitudeRange :type Float%20Range%20Structure) (PlayerLatitude :type Float%20%28single-precision%29) (PlayerLongitude :type Float%20%28single-precision%29))
  (return (Utilities|CalculateLocation PlayerLatitude LocationLatitudeRange PlayerLongitude LocationLongitudeRange)))

(fn BreakCoordinateRanges
  (params (CoordinateRange :type Float%20Range%20Structure))
  (bind (_lowerbound _upperbound) (Utilities|Struct|BreakFloatRange CoordinateRange))
  (return (.Value (Utilities|Struct|BreakFloatRangeBound _lowerbound)) (.Value (Utilities|Struct|BreakFloatRangeBound _upperbound))))