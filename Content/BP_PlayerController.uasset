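; Player controller for a location-based fairy-befriending game, acting as the hub for GPS checks and save data.
; On BeginPlay it constructs logger, checker and saver objects, feeding refreshed coordinates into location-range checks.
; Befriending saves new friendships and records the latest fairy on the game instance.
; It also broadcasts touch and app-backgrounding events, and toggles a debug menu via repeated three-finger touches or the D key.
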(event ApplicationWillEnterBackgroundDelegate(ApplicationLifecycle)
  (Default|CallOnBackgroundEntered))

(event Custom|Toggle%20Debug%20Menu
  ;[1 1 1] Toggles the debug menu on and off.
  (bind _foundwidgets (Widget|GetAllWidgetsOfClass "/Game/Widgets/WBP_DebugMenu.WBP_DebugMenu_C" true))
  (if (> (Utilities|Array|Length _foundwidgets) 0)
    (Widget|RemovefromParent _foundwidgets)
    (else
      (bind _returnvalue (UserInterface|CreateWidget "/Game/Widgets/WBP_DebugMenu.WBP_DebugMenu_C" (Game|GetPlayerController 0)))
      (UserInterface|Viewport|AddtoViewport _returnvalue 0))))

(event Custom|TouchScreenDebug
  (params (FingerIndex :type ETouchIndex%20Enum :default "Touch1"))
  ;[1 1 1] Toggles debug menu only if 3 fingers touch the screen 2 times.
  (switch Utilities|FlowControl|Switch|SwitchonETouchIndex FingerIndex
    (:Touch3
      (switch int (Variables|Default|GetDebugIndex)
        (:Default
          ;[1 1 1] Resets debug index after a 1 second delay.
          (Math|Integer|IncrementInt (Variables|Default|GetDebugIndex)
            (:%20%20
              (Utilities|FlowControl|Delay 1.0)
              (Variables|Default|SetDebugIndex 0))))
        (:4
          (CallFunction|ToggleDebugMenu)
          (Variables|Default|SetDebugIndex 0))))))

(event EventBeginPlay
  (bind _returnvalue (Game|ConstructObjectfromClass "/Game/BP_GPSLogger.BP_GPSLogger_C" self))
  (bind _output_get (Variables|Default|SetGPSLogger _returnvalue))
  (Default|GPSFirstTimeStartup _output_get)
  (bind _returnvalue_2 (Game|ConstructObjectfromClass "/Game/BP_GPSChecker.BP_GPSChecker_C" self))
  (Variables|Default|SetGPSChecker _returnvalue_2)
  (bind _returnvalue_3 (Game|ConstructObjectfromClass "/Game/BP_GameSaver.BP_GameSaver_C" self))
  (bind _output_get_2 (Variables|Default|SetGame%20Saver _returnvalue_3))
  (Default|LoadSavefromMemory _output_get_2))

(event Input|KeyboardEvents|D
  (params (Key :type Key%20Structure))
  ;[1 1 1] Toggles Debug Menu if * key is pressed.
  (:Pressed
    (CallFunction|ToggleDebugMenu)))

(event Input|TouchEvents|InputTouch
  (params (Location :type Vector) (FingerIndex :type ETouchIndex%20Enum))
  (:Pressed
    (Default|CallOnScreenTouched)
    (CallFunction|TouchScreenDebug FingerIndex)))

(fn ConstructionScript)

(fn IsPlayeratLocation
  (params (LocationLatitudeRange :type Float%20Range%20Structure) (LocationLongitudeRange :type Float%20Range%20Structure))
  (bind _gpslogger (Variables|Default|GetGPSLogger))
  (Default|RefreshLocation _gpslogger)
  (bind _isatlocation (Default|IsPlayeratLocation (Variables|Default|GetGPSChecker) LocationLatitudeRange LocationLongitudeRange (Variables|/Game/BP_GPSLogger.BP_GPSLogger_C|GetLatitude _gpslogger) (Variables|/Game/BP_GPSLogger.BP_GPSLogger_C|GetLongitude _gpslogger)))
  (return _isatlocation))

(fn BefriendFairy
  (params (Fairy :type eFairy%20Enum :default "NewEnumerator3"))
  (bind _game_saver (Variables|Default|GetGame%20Saver))
  (bind _isfriend (Default|GetIsFriendswith _game_saver Fairy))
  (if (not _isfriend)
    (Default|SetFairyasFriend _game_saver Fairy true)
    (bind _asbp_game_instance (Utilities|Casting|CastToBP_GameInstance (Game|GetGameInstance)))
    (Variables|/Game/BP_GameInstance.BP_GameInstance_C|SetMostRecentlyFoundFairy _asbp_game_instance Fairy)))

(fn DeleteSave
  (Default|DeleteSaveData (Variables|Default|GetGame%20Saver)))

(fn IsFriendswithAllFairies
  (bind _result (Default|AllFairiesFriended (Variables|Default|GetGame%20Saver)))
  (return _result))